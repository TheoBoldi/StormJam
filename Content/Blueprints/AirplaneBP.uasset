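; Airplane actor that flies across the level in one of three random variants, each carrying its own point reward.
; On BeginPlay it picks a variant, setting its size enum, points, mesh and engine audio pitch, with lower pitch for larger rewards.
; Tick moves it along its right vector at Speed without sweeping, and it destroys itself after a fixed delay shared by all variants.
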(event `self.ReceiveBeginPlay`
  (bind _airplaneaudio (`self.AirplaneAudio`))
  (bind _airplaneaudio_2 (`self.AirplaneAudio`))
  (bind _airplaneaudio_3 (`self.AirplaneAudio`))
  (set `self.Location` (`self.K2_GetActorLocation`))
  (switch `int` (`KismetMathLibrary.RandomInteger` 3)
    (:`0`
      (set `self.Size` "NewEnumerator0")
      (set `self.Points` (`self.SmallReward`))
      (`StaticMeshComponent.SetStaticMesh` (`self.StaticMesh`) "/Game/ART/airplane1_airplane_3.airplane1_airplane_3")
      (`AudioComponent.Play` _airplaneaudio_2 0.0)
      (`AudioComponent.SetPitchMultiplier` _airplaneaudio_2 1.2))
    (:`1`
      (set `self.Size` "NewEnumerator1")
      (set `self.Points` (`self.MediumReward`))
      (`StaticMeshComponent.SetStaticMesh` (`self.StaticMesh`) "/Game/ART/airplane1_airplane_2.airplane1_airplane_2")
      (`AudioComponent.Play` _airplaneaudio_3 0.0)
      (`AudioComponent.SetPitchMultiplier` _airplaneaudio_3 1.0))
    (:`2`
      (set `self.Size` "NewEnumerator2")
      (set `self.Points` (`self.LargeReward`))
      (`StaticMeshComponent.SetStaticMesh` (`self.StaticMesh`) "/Game/ART/airplane1_aiplane_1.airplane1_aiplane_1")
      (`AudioComponent.Play` _airplaneaudio 0.0)
      (`AudioComponent.SetPitchMultiplier` _airplaneaudio 0.8)))
  (`KismetSystemLibrary.Delay` 60.0)
  (`self.K2_DestroyActor`))

(event `self.ReceiveTick`
  (params (DeltaSeconds :type "Float (single-precision)"))
  (bind _output_get (set `self.Location` (+ (`self.Location`) (* (* (`self.GetActorRightVector`) (`self.Speed`)) DeltaSeconds))))
  (`self.K2_SetActorLocation` _output_get))

(fn `UserConstructionScript`)